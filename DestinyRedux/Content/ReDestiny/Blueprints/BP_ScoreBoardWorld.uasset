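; World-placed scoreboard Blueprint that displays a BasicScoreboard widget through its ScoreBoardWidget component.
; On BeginPlay it casts the component's user widget to BasicScoreboard and stores the reference.
; It then fills the board with ten debug entries, each using one random number for both the player name and the score.
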(event `self.ReceiveBeginPlay`
  (bind _asbasic_scoreboard (cast `/Game/ReDestiny/Widgets/ScoreBoard/BasicScoreboard` (`WidgetComponent.GetUserWidgetObject` (`self.ScoreBoard_Widget`))))
  (set `self.ScoreboardRef` _asbasic_scoreboard)
  (`self.Debug_AddRandScores`))

(fn `Debug_AddRandScores`
  (locals (localRandInt :type Integer))
  (for _ (range 10)
    (set `local.localRandInt` (`KismetMathLibrary.RandomInteger` 10000000))
    (`/Game/ReDestiny/Widgets/ScoreBoard/BasicScoreboard.AddScore` (`self.ScoreboardRef`) (make `/Game/ReDestiny/Blueprints/Structs/S_ScoreBoard` (`|FormatText` "Player{num}" (`KismetTextLibrary.Conv_IntToText` (`local.localRandInt`) false)) (`local.localRandInt`))))
  (return))

(fn `UserConstructionScript`)