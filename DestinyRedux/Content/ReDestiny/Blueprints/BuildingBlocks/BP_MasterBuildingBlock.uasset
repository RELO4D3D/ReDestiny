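; Base building block that shows when its required-space volume is overlapped by swapping its mesh to an overlap material.
; On BeginPlay it caches original materials and flags existing overlaps, skipping specific stair and floor classes.
; ReqSpace overlap events, filtered by I_SpaceRequirements but not by class, track overlapping actors.
; Each slot gets a dynamic M_Overlapping instance, and originals return once that list empties.
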(event `CheckOverlaps`
  (if (not (`self.shouldCollide` self))
    (for _array_element (`PrimitiveComponent.GetOverlappingActors` (`self.ReqSpace`) null)
      (if (!= _array_element self)
        (if (not (`self.shouldCollide` _array_element))
          (`KismetSystemLibrary.PrintString` (`KismetTextLibrary.Conv_TextToString` (`|FormatText` (`KismetTextLibrary.Conv_StringToText` (`KismetSystemLibrary.GetDisplayName` self)) "{self} is overlapped by {that}" (`KismetTextLibrary.Conv_StringToText` (`KismetSystemLibrary.GetDisplayName` _array_element)))) true true (struct :`G` 0.66 :`B` 1.0 :`A` 1.0) 10.0)
          (`self.OnOverlapStart`))))))

(event `self.ReceiveBeginPlay`
  (set `self.OrigMats` (`MeshComponent.GetMaterials` (`self.StaticMesh`)))
  (`self.CheckOverlaps`))

(event `/Game/ReDestiny/Blueprints/Interfaces/I_SpaceRequirements.OnOverlapStart`
  (for (_array_element _array_index) (`self.OrigMats`)
    (bind _returnvalue (`KismetMaterialLibrary.CreateDynamicMaterialInstance` _array_element "/Game/ReDestiny/Materials/Testing/M_Overlapping.M_Overlapping"))
    (`PrimitiveComponent.SetMaterial` (`self.StaticMesh`) _array_index _returnvalue)))

(event `/Game/ReDestiny/Blueprints/Interfaces/I_SpaceRequirements.OnOverlapEnd`
  (for (_array_element _array_index) (`self.OrigMats`)
    (`PrimitiveComponent.SetMaterial` (`self.StaticMesh`) _array_index _array_element)))

(event `self.ReqSpace.OnComponentBeginOverlap`
  (params (OverlappedComponent :type "PrimitiveComponent Object Reference") (OtherActor :type "Actor Object Reference") (OtherComp :type "PrimitiveComponent Object Reference") (OtherBodyIndex :type Integer) (bFromSweep :type Boolean) (SweepResult :type "HitResult Structure (by ref)"))
  (if (`KismetSystemLibrary.DoesImplementInterface` OtherActor "/Game/ReDestiny/Blueprints/Interfaces/I_SpaceRequirements.I_SpaceRequirements_C")
    (if (< (`KismetArrayLibrary.Array_Length` (`self.OrigMats`)) 1)
      (set `self.OrigMats` (`MeshComponent.GetMaterials` (`self.StaticMesh`))))
    (`KismetArrayLibrary.Array_AddUnique` (`self.OverlappingActors`) null)
    (`self.OnOverlapStart`)))

(event `self.ReqSpace.OnComponentEndOverlap`
  (params (OverlappedComponent :type "PrimitiveComponent Object Reference") (OtherActor :type "Actor Object Reference") (OtherComp :type "PrimitiveComponent Object Reference") (OtherBodyIndex :type Integer))
  (bind _overlappingactors (`self.OverlappingActors`))
  (if (`KismetSystemLibrary.DoesImplementInterface` OtherActor "/Game/ReDestiny/Blueprints/Interfaces/I_SpaceRequirements.I_SpaceRequirements_C")
    (`KismetArrayLibrary.Array_RemoveItem` _overlappingactors OtherActor)
    (if (not (> (`KismetArrayLibrary.Array_Length` _overlappingactors) 0))
      (`self.OnOverlapEnd`))))

(event `OnOverlap_Materials`
  (params (inActor :type Boolean)))

(fn `isFloorClass`
  (params (inActor :type "Actor Object Reference"))
  (returns (isFloor :type Boolean))
  (bind _returnvalue (`GameplayStatics.GetObjectClass` inActor))
  (return (or (== _returnvalue "/Game/ReDestiny/Blueprints/BuildingBlocks/Floors/BP_Floor_10x10.BP_Floor_10x10_C") (== _returnvalue "/Game/ReDestiny/Blueprints/BuildingBlocks/Floors/BP_Floor_50x50.BP_Floor_50x50_C"))))

(fn `isStairsClass`
  (params (inActor :type "Actor Object Reference"))
  (returns (isStairs :type Boolean))
  (return (== (`GameplayStatics.GetObjectClass` inActor) "/Game/ReDestiny/Blueprints/BuildingBlocks/Stairs/BP_Stairs_Straight_Open_2x9.BP_Stairs_Straight_Open_2x9_C")))

(fn `shouldCollide`
  (params (inActor :type "Actor Object Reference"))
  (returns (isProtectedCollider :type Boolean))
  (return (or (`self.isStairsClass` inActor) (`self.isFloorClass` inActor))))

(fn `UserConstructionScript`)