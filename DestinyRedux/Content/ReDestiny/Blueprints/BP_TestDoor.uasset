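; BP_TestDoor is an automatic sliding double door with trigger boxes in front and behind.
; Entering either box plays a timeline that slides both panels in opposite directions from positions cached at BeginPlay, scaled by OpenAmount.
; Leaving either box reverses the timeline from its end after a fixed delay, lengthened if the door is not yet almost fully open.
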(event `self.ReceiveBeginPlay`
  (set `self.LeftDoorPos` (`SceneComponent.RelativeLocation` (`self.Door_Left`)))
  (set `self.RightDoorPos` (`SceneComponent.RelativeLocation` (`self.Door_Right`))))

(event `self.BoxTrigger_Front.OnComponentBeginOverlap`
  (params (OverlappedComponent :type "PrimitiveComponent Object Reference") (OtherActor :type "Actor Object Reference") (OtherComp :type "PrimitiveComponent Object Reference") (OtherBodyIndex :type Integer) (bFromSweep :type Boolean) (SweepResult :type "HitResult Structure (by ref)"))
  (bind (_direction _opentiming) (`Timeline|Door_Timeline` :!label _label)
    (:`Update`
      (bind _returnvalue (* (`self.OpenAmount`) _opentiming))
      (`SceneComponent.K2_SetRelativeLocation` (`self.Door_Left`) (- (`self.LeftDoorPos`) _returnvalue) false true)
      (`SceneComponent.K2_SetRelativeLocation` (`self.Door_Right`) (+ (`self.RightDoorPos`) _returnvalue) false true))))

(event `self.BoxTrigger_Back.OnComponentBeginOverlap`
  (params (OverlappedComponent :type "PrimitiveComponent Object Reference") (OtherActor :type "Actor Object Reference") (OtherComp :type "PrimitiveComponent Object Reference") (OtherBodyIndex :type Integer) (bFromSweep :type Boolean) (SweepResult :type "HitResult Structure (by ref)"))
  (goto _label))

(event `self.BoxTrigger_Front.OnComponentEndOverlap`
  (params (OverlappedComponent :type "PrimitiveComponent Object Reference") (OtherActor :type "Actor Object Reference") (OtherComp :type "PrimitiveComponent Object Reference") (OtherBodyIndex :type Integer))
  (if (not (>= (stale `self.BoxTrigger_Front.OnComponentBeginOverlap` _opentiming) 0.95)) :!label _label_2
    (`KismetSystemLibrary.Delay` 2.1))
  (`KismetSystemLibrary.Delay` 5.0)
  (goto _label :!via `ReverseFromEnd`))

(event `self.BoxTrigger_Back.OnComponentEndOverlap`
  (params (OverlappedComponent :type "PrimitiveComponent Object Reference") (OtherActor :type "Actor Object Reference") (OtherComp :type "PrimitiveComponent Object Reference") (OtherBodyIndex :type Integer))
  (goto _label_2))

(fn `UserConstructionScript`)