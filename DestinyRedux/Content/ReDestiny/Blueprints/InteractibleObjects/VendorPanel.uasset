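; VendorPanel is an interactable world actor that shows a full-screen vendor widget while the player stands near it.
; Its box collision overlaps filter for actors implementing I_Interactible that cast to FirstPersonCharacter, then fire the enter and leave radius events.
; Entering lazily creates and caches the FullScreenVendorWidget for player 0 and adds it to the viewport, and leaving removes it.
; The OnInteractwith event is left empty, so proximity alone drives the panel.
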(event `self.BoxCollision.OnComponentBeginOverlap`
  (params (OverlappedComponent :type "PrimitiveComponent Object Reference") (OtherActor :type "Actor Object Reference") (OtherComp :type "PrimitiveComponent Object Reference") (OtherBodyIndex :type Integer) (bFromSweep :type Boolean) (SweepResult :type "HitResult Structure (by ref)"))
  (if (`KismetSystemLibrary.DoesImplementInterface` OtherActor "/Game/ReDestiny/Blueprints/Interfaces/I_Interactible.I_Interactible_C")
    (bind _asfirst_person_character (cast `/Game/FirstPersonBP/Blueprints/FirstPersonCharacter` OtherActor))
    (`/Game/ReDestiny/Blueprints/Interfaces/I_Interactible.OnEnterPlayerRadius` _asfirst_person_character)))

(event `self.BoxCollision.OnComponentEndOverlap`
  (params (OverlappedComponent :type "PrimitiveComponent Object Reference") (OtherActor :type "Actor Object Reference") (OtherComp :type "PrimitiveComponent Object Reference") (OtherBodyIndex :type Integer))
  (if (`KismetSystemLibrary.DoesImplementInterface` OtherActor "/Game/ReDestiny/Blueprints/Interfaces/I_Interactible.I_Interactible_C")
    (bind _asfirst_person_character (cast `/Game/FirstPersonBP/Blueprints/FirstPersonCharacter` OtherActor))
    (`/Game/ReDestiny/Blueprints/Interfaces/I_Interactible.OnLeavePlayerRadius` _asfirst_person_character)))

(event `/Game/ReDestiny/Blueprints/Interfaces/I_Interactible.OnInteractWith`
  (params (Character :type "/Game/FirstPersonBP/Blueprints/FirstPersonCharacter Object Reference")))

(event `/Game/ReDestiny/Blueprints/Interfaces/I_Interactible.OnEnterPlayerRadius`
  (params (Character :type "/Game/FirstPersonBP/Blueprints/FirstPersonCharacter Object Reference"))
  (bind _vendorpanelinteractionref (`self.VendorPanelInteractionRef`))
  (`/Engine/EditorBlueprintResources/StandardMacros.IsValid` (`self.PlayerControllerRef`)
    (:`Is Valid`
      _)
    (:`Is Not Valid`
      (set `self.PlayerControllerRef` (`GameplayStatics.GetPlayerController` 0))))
  (`/Engine/EditorBlueprintResources/StandardMacros.IsValid` _vendorpanelinteractionref
    (:`Is Valid`
      _)
    (:`Is Not Valid`
      (bind _returnvalue (`|CreateWidget` "/Game/ReDestiny/Widgets/VendorSections/FullScreenVendorWidget.FullScreenVendorWidget_C" (`self.PlayerControllerRef`)))
      (set `self.VendorPanelInteractionRef` _returnvalue)))
  (if (not (`Widget.IsInViewport` _vendorpanelinteractionref))
    (`UserWidget.AddToViewport` (`self.VendorPanelInteractionRef`) 0)))

(event `/Game/ReDestiny/Blueprints/Interfaces/I_Interactible.OnLeavePlayerRadius`
  (params (Character :type "/Game/FirstPersonBP/Blueprints/FirstPersonCharacter Object Reference"))
  (bind _vendorpanelinteractionref (`self.VendorPanelInteractionRef`))
  (if (`Widget.IsInViewport` _vendorpanelinteractionref)
    (`Widget.RemoveFromParent` _vendorpanelinteractionref)))

(fn `UserConstructionScript`)