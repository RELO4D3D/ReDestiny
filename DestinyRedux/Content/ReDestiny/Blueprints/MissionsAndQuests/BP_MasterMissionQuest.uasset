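; Master Blueprint for missions and quests, tracking progress through numbered steps that each map to a group of substeps.
; Starting a step sets its substeps' statuses; completing all of them advances to the next step, or calls an empty completion stub when none remains.
; EnsureSanity resizes the status array and reloads current substeps from the clamped step.
; AutomationTests asserts that step and substep definitions are consistent.
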(fn `AutomationTests`
  (locals (TempIntSum :type Integer) (HighestSubstepIndex :type Integer) (HighestStepIndex :type Integer))
  (bind _functionaltestref (`self.FunctionalTestRef`))
  (`FunctionalTest.AssertTrue` _functionaltestref (< (`self.Default_CurrentStep`) (`BlueprintMapLibrary.Map_Length` (`.SubstepsPerStep_34_764085D9414C5512173FFF803CB2097D` (break `/Game/ReDestiny/Blueprints/Structs/S_MissionQuest` (`self.Default_MissionQuestInfo`))))) "Assertion Failed: Cannot allow 'Current Step' to be greater than the number of steps defined for this Mission/Quest.")
  (bind _values (`BlueprintMapLibrary.Map_Values` (`.SubstepsPerStep_34_764085D9414C5512173FFF803CB2097D` (break `/Game/ReDestiny/Blueprints/Structs/S_MissionQuest` (`self.Default_MissionQuestInfo`)))))
  (for (_array_element _array_index) _values
    (bind _output_get (set `local.TempIntSum` (+ (`KismetArrayLibrary.Array_Length` (`.IntArray_6_08D7AA7348557B3F197450BE323BE770` (break `/Game/ReDestiny/Blueprints/Structs/S_GenericIntArray` _array_element))) (`local.TempIntSum`))))
    (set `local.HighestSubstepIndex` (- _output_get 1))
    (set `local.HighestStepIndex` (+ _array_index 1)))
  (`FunctionalTest.AssertTrue` _functionaltestref (== (`local.TempIntSum`) (`KismetArrayLibrary.Array_Length` (`.Substeps_29_AAF74A1640B02658F479A4BA3A957D04` (break `/Game/ReDestiny/Blueprints/Structs/S_MissionQuest` (`self.Default_MissionQuestInfo`))))) "Assertion Failed: Mismatch between number of defined steps in 'MissionQuestInfo' and the number of substeps defined for this Mission/Quest.")
  (`FunctionalTest.AssertTrue` _functionaltestref (`KismetArrayLibrary.Array_Contains` (`.IntArray_6_08D7AA7348557B3F197450BE323BE770` (break `/Game/ReDestiny/Blueprints/Structs/S_GenericIntArray` (`BlueprintMapLibrary.Map_Find` (`.SubstepsPerStep_34_764085D9414C5512173FFF803CB2097D` (break `/Game/ReDestiny/Blueprints/Structs/S_MissionQuest` (`self.Default_MissionQuestInfo`))) (`local.HighestStepIndex`)))) (`local.HighestSubstepIndex`)) "Assertion Failed: Ordering of steps in 'MissionQuestInfo' may be unordered for this Mission/Quest. Alternatively, modify 'SubstepsPerStep' to ensure the final step defined in 'MissionQuestInfo' is the final stubstep expected to complete this Mission/Quest. Consider ordering them sequentially for readability and sanity.")
  (return))

(fn `CompleteMissionQuest(Stub)`
  (return))

(fn `CompleteSubstep`
  (params (SubstepIndex :type Integer))
  (`self.UpdateSubstepStatus` SubstepIndex "NewEnumerator1")
  (for _array_element (`self.Default_CurrentSubsteps`)
    (if (`|EnumInequality` (`KismetArrayLibrary.Array_Get` (`self.Default_SubstepStatuses`) _array_element) "NewEnumerator1")
      (return)))
  (bind _result (`/Engine/EditorBlueprintResources/StandardMacros.IncrementInt` (`self.Default_CurrentStep`))
    (:`  `
      (`self.UpdateCurrentSubsteps` _result)
      (return))))

(fn `EnsureSanity`
  (bind ((`DescriptionsPerStep_45_15D80D184978E964CBA818BD29849F37` _descriptionsperstep) (`SubstepsPerStep_34_764085D9414C5512173FFF803CB2097D` _substepsperstep)) (break `/Game/ReDestiny/Blueprints/Structs/S_MissionQuest` (`self.Default_MissionQuestInfo`)))
  (bind _returnvalue (`KismetArrayLibrary.Array_Length` (`.Substeps_29_AAF74A1640B02658F479A4BA3A957D04` (break `/Game/ReDestiny/Blueprints/Structs/S_MissionQuest` (`self.Default_MissionQuestInfo`)))))
  (if (not (== _returnvalue (`KismetArrayLibrary.Array_Length` (`self.Default_SubstepStatuses`))))
    (`KismetArrayLibrary.Array_Resize` (`self.Default_SubstepStatuses`) _returnvalue))
  (set `self.Default_CurrentSubsteps` (`.IntArray_6_08D7AA7348557B3F197450BE323BE770` (break `/Game/ReDestiny/Blueprints/Structs/S_GenericIntArray` (`BlueprintMapLibrary.Map_Find` _substepsperstep (`KismetMathLibrary.Clamp` (`self.Default_CurrentStep`) 1 (`BlueprintMapLibrary.Map_Length` _substepsperstep))))))
  (return))

(fn `InitMissionQuest`
  (`self.UpdateCurrentSubsteps` 1)
  (return))

(fn `UpdateCurrentSubsteps`
  (params (NewStep :type Integer))
  (bind (_value _returnvalue) (`BlueprintMapLibrary.Map_Find` (`.SubstepsPerStep_34_764085D9414C5512173FFF803CB2097D` (break `/Game/ReDestiny/Blueprints/Structs/S_MissionQuest` (`self.Default_MissionQuestInfo`))) NewStep))
  (if _returnvalue
    (bind _output_get (set `self.Default_CurrentSubsteps` (`.IntArray_6_08D7AA7348557B3F197450BE323BE770` (break `/Game/ReDestiny/Blueprints/Structs/S_GenericIntArray` _value))))
    (for _array_element _output_get
      (`self.UpdateSubstepStatus` _array_element "NewEnumerator0"))
    (return)
    (else
      (`self.CompleteMissionQuest(Stub)`)
      (return))))

(fn `UpdateSubstepStatus`
  (params (SubstepIndex :type Integer) (NewTaskStatus :type "/Game/ReDestiny/Blueprints/Enums/E_TaskStatus Enum"))
  (`KismetArrayLibrary.Array_Set` (`self.Default_SubstepStatuses`) SubstepIndex NewTaskStatus)
  (return))

(fn `UserConstructionScript`)